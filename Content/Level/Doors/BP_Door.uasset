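; BP_Door is an interactable door that can be open, closed or locked behind a key item.
; Entering its Box binds OnInteract to the first-person character, unless the door is locked and the key is missing, and shows a state-based WP_Interact prompt.
; Interacting toggles the Cube's visibility and collision instead of animating it, updating the state and prompt visibility.
; Leaving the Box hides the prompt and unbinds the interaction.
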(event OnComponentBeginOverlap(Box)
  (params (OverlappedComponent :type Primitive%20Component%20Object%20Reference) (OtherActor :type Actor%20Object%20Reference) (OtherComp :type Primitive%20Component%20Object%20Reference) (OtherBodyIndex :type Integer) (bFromSweep :type Boolean) (SweepResult :type Hit%20Result%20Structure%20%28by%20ref%29))
  (bind _interactcomponent (Variables|Default|GetInteractComponent))
  (bind _asbp_first_person_character (Utilities|Casting|CastToBP_FirstPersonCharacter OtherActor))
  (Variables|Default|SetPlayer _asbp_first_person_character)
  (if (or (Utilities|Enum|NotEqual(Enum) (Variables|Default|GetState) "NewEnumerator1") (Default|HasItem _asbp_first_person_character (Variables|Default|GetKey)))
    (EventDispatchers|BindEventtoOnInteract _asbp_first_person_character (delegate Custom|On%20Interact)))
  (if (Utilities|IsValid (UserInterface|GetWidget (Variables|Default|GetInteractComponent)))
    (switch Utilities|FlowControl|Switch|SwitchonE_States (Variables|Default|GetState)
      (:NewEnumerator0
        (Variables|/Game/UI/WP_Interact.WP_Interact_C|SetText (Variables|Default|GetInteractWidget) "[E] Close"))
      (:NewEnumerator1
        (if (Default|HasItem (Variables|Default|GetPlayer) (Variables|Default|GetKey))
          (Variables|/Game/UI/WP_Interact.WP_Interact_C|SetText (Variables|Default|GetInteractWidget) "[E] Unlock Door")
          (else
            (Variables|/Game/UI/WP_Interact.WP_Interact_C|SetText (Variables|Default|GetInteractWidget) "Locked"))))
      (:NewEnumerator2
        (Variables|/Game/UI/WP_Interact.WP_Interact_C|SetText (Variables|Default|GetInteractWidget) "[E] Open")))
    (Widget|SetVisibility (UserInterface|GetWidget (Variables|Default|GetInteractComponent)) "Visible")
    (else
      (bind _returnvalue (UserInterface|CreateWidget "/Game/UI/WP_Interact.WP_Interact_C" (Game|GetPlayerController 0)))
      (bind _output_get (Variables|Default|SetInteractWidget _returnvalue))
      (switch Utilities|FlowControl|Switch|SwitchonE_States (Variables|Default|GetState)
        (:NewEnumerator0
          (Variables|/Game/UI/WP_Interact.WP_Interact_C|SetText _output_get "[E] Close"))
        (:NewEnumerator1
          (if (Default|HasItem (Variables|Default|GetPlayer) (Variables|Default|GetKey))
            (Variables|/Game/UI/WP_Interact.WP_Interact_C|SetText _output_get "[E] Unlock Door")
            (else
              (Variables|/Game/UI/WP_Interact.WP_Interact_C|SetText _output_get "Locked"))))
        (:NewEnumerator2
          (Variables|/Game/UI/WP_Interact.WP_Interact_C|SetText _output_get "[E] Open")))
      (UserInterface|SetWidget _interactcomponent _output_get)
      (Components|Activation|Activate _interactcomponent false)
      (Widget|Transform|SetRenderScale (Variables|Default|GetInteractWidget) "(X=2.000000,Y=2.000000)"))))

(event OnComponentEndOverlap(Box)
  (params (OverlappedComponent :type Primitive%20Component%20Object%20Reference) (OtherActor :type Actor%20Object%20Reference) (OtherComp :type Primitive%20Component%20Object%20Reference) (OtherBodyIndex :type Integer))
  (bind _asbp_first_person_character (Utilities|Casting|CastToBP_FirstPersonCharacter OtherActor))
  (Widget|SetVisibility (Variables|Default|GetInteractWidget) "Hidden")
  (EventDispatchers|UnbindallEventsfromOnInteract _asbp_first_person_character))

(event Custom|On%20Interact
  (bind _cube (Variables|Default|GetCube))
  (if (Variables|Default|GetOpen)
    (Rendering|SetVisibility _cube true false)
    (Collision|SetCollisionEnabled _cube "QueryAndPhysics")
    (Widget|SetVisibility (Variables|Default|GetInteractWidget) "Visible")
    (Variables|Default|SetOpen false)
    (Variables|Default|SetState "NewEnumerator2")
    (else
      (Rendering|SetVisibility _cube false false)
      (Collision|SetCollisionEnabled _cube "NoCollision")
      (Widget|SetVisibility (Variables|Default|GetInteractWidget) "Hidden")
      (Variables|Default|SetOpen true)
      (Variables|Default|SetState "NewEnumerator0"))))

(event EventBeginPlay)

(event Collision|EventActorBeginOverlap
  (params (OtherActor :type Actor%20Object%20Reference)))

(event EventTick
  (params (DeltaSeconds :type Float%20%28single-precision%29)))

(fn ConstructionScript)