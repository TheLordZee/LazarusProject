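; BP_Item is a world item that the first-person character can pick up into its inventory.
; When that character overlaps the collision, the item binds its Pickup event to the character's OnInteract and shows an interact prompt, creating the WP_Interact widget on InteractComponent if none exists.
; Pickup passes the item to the character's BPInventoryComponent.
; No end-overlap logic unbinds the event or hides the prompt.
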(event OnComponentBeginOverlap(Collision)
  (params (OverlappedComponent :type Primitive%20Component%20Object%20Reference) (OtherActor :type Actor%20Object%20Reference) (OtherComp :type Primitive%20Component%20Object%20Reference) (OtherBodyIndex :type Integer) (bFromSweep :type Boolean) (SweepResult :type Hit%20Result%20Structure%20%28by%20ref%29))
  (bind _interactcomponent (Variables|Default|GetInteractComponent))
  (bind _asbp_first_person_character (Utilities|Casting|CastToBP_FirstPersonCharacter OtherActor))
  (EventDispatchers|BindEventtoOnInteract _asbp_first_person_character (delegate Custom|Pickup))
  (if (Utilities|IsValid (UserInterface|GetWidget (Variables|Default|GetInteractComponent)))
    (Widget|SetVisibility (UserInterface|GetWidget (Variables|Default|GetInteractComponent)) "Visible")
    (else
      (bind _returnvalue (UserInterface|CreateWidget "/Game/UI/WP_Interact.WP_Interact_C" (Game|GetPlayerController 0)))
      (Variables|Default|SetInteractWidget _returnvalue)
      (UserInterface|SetWidget _interactcomponent _returnvalue)
      (Components|Activation|Activate _interactcomponent false)
      (Widget|Transform|SetRenderScale (Variables|Default|GetInteractWidget) "(X=2.000000,Y=2.000000)"))))

(event Custom|Pickup
  (Default|Pickup (Variables|/Game/Player/Blueprints/BP_FirstPersonCharacter.BP_FirstPersonCharacter_C|GetBP_InventoryComponent (stale OnComponentBeginOverlap(Collision) _asbp_first_person_character)) self))

(event EventBeginPlay)

(event Collision|EventActorBeginOverlap
  (params (OtherActor :type Actor%20Object%20Reference)))

(event EventTick
  (params (DeltaSeconds :type Float%20%28single-precision%29)))

(fn ConstructionScript)